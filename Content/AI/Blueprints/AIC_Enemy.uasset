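; AI controller for enemies that runs BT_Enemy on possession and tracks the player through AI perception.
; Sensing an actor tagged Player cancels the lost-sight timer and writes HasLineOfSight and TargetActor to the blackboard.
; Losing the player clears HasLineOfSight immediately but keeps the target for an eight-second grace period before LostSight empties TargetActor.
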(event `self.ReceivePossess`
  (params (PossessedPawn :type "Pawn Object Reference"))
  (`self.RunBehaviorTree` "/Game/AI/Blueprints/BT_Enemy.BT_Enemy"))

(event `self.AIPerception.OnTargetPerceptionUpdated`
  (params (Actor :type "Actor Object Reference") (Stimulus :type "AIStimulus Structure"))
  (set `self.Perceived Actor` Actor)
  (if (`self.ActorHasTag` Actor "Player")
    (if (`.bSuccessfullySensed` (break `AIStimulus` Stimulus))
      (`KismetSystemLibrary.K2_ClearAndInvalidateTimerHandle` (`self.Lost Sight Timer`))
      (`self.UpdateSightKey` true)
      (`self.UpdateTargetKey` (`self.Perceived Actor`))
      (else
        (bind _returnvalue (`KismetSystemLibrary.K2_SetTimerDelegate` (delegate `LostSight`) 8.0))
        (set `self.Lost Sight Timer` _returnvalue)
        (`self.UpdateSightKey` false)))))

(event `LostSight`
  (`self.UpdateTargetKey` null))

(fn `UpdateSightKey`
  (params (HasLineOfSight :type Boolean))
  (`BlackboardComponent.SetValueAsBool` (`self.Blackboard`) "HasLineOfSight" HasLineOfSight))

(fn `UpdateTargetKey`
  (params (TargetActor :type "Actor Object Reference"))
  (`BlackboardComponent.SetValueAsObject` (`self.Blackboard`) "TargetActor" TargetActor))

(fn `UserConstructionScript`)